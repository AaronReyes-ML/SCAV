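; InteriorWindRegion is a trigger volume that changes the wind level while the first-person character is inside it.
; On BeginPlay it finds the B_WindSystem actor and expires after a brief lifespan if none exists.
; Box overlap by a FirstPersonCharacter passes the region's level L to SetWindLevel, and leaving passes -1.
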(event OnComponentBeginOverlap(Box)
  (params (OverlappedComponent :type Primitive%20Component%20Object%20Reference) (OtherActor :type Actor%20Object%20Reference) (OtherComp :type Primitive%20Component%20Object%20Reference) (OtherBodyIndex :type Integer) (bFromSweep :type Boolean) (SweepResult :type Hit%20Result%20Structure%20%28by%20ref%29))
  (Utilities|Casting|CastToFirstPersonCharacter OtherActor)
  (Default|SetWindLevel (Variables|Default|GetWind) (Variables|Default|GetL)))

(event OnComponentEndOverlap(Box)
  (params (OverlappedComponent :type Primitive%20Component%20Object%20Reference) (OtherActor :type Actor%20Object%20Reference) (OtherComp :type Primitive%20Component%20Object%20Reference) (OtherBodyIndex :type Integer))
  (Utilities|Casting|CastToFirstPersonCharacter OtherActor)
  (Default|SetWindLevel (Variables|Default|GetWind) -1))

(event EventBeginPlay
  (bind _returnvalue (Actor|GetActorOfClass "/Game/Audio/Blueprints/B_WindSystem.B_WindSystem_C"))
  (bind _output_get (Variables|Default|SetWind _returnvalue))
  (Utilities|IsValid _output_get
    (:Is%20Not%20Valid
      (Actor|SetLifeSpan 0.1))))

(event Collision|EventActorBeginOverlap
  (params (OtherActor :type Actor%20Object%20Reference)))

(event EventTick
  (params (DeltaSeconds :type Float%20%28single-precision%29)))

(fn ConstructionScript)