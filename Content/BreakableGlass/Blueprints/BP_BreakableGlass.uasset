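; Breakable glass pane actor in three sizes, with optional shadows, that shatters from impacts or multicast explosive damage.
; The construction script builds a grid of hit boxes tagged with cell index and row/column.
; FirstHitPositionObject swaps in that cell's pre-fractured destructible mesh, applies radial damage, sound and particles, and optionally offsets break normals to match.
; Later hits add damage; delayed follow-ups collapse remaining pieces and disable collision.
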(event OnComponentHit(SM_Glass_DM)
  (params (HitComponent :type Primitive%20Component%20Object%20Reference) (OtherActor :type Actor%20Object%20Reference) (OtherComp :type Primitive%20Component%20Object%20Reference) (NormalImpulse :type Vector :default "0, 0, 0") (Hit :type Hit%20Result%20Structure%20%28by%20ref%29))
  (bind _returnvalue (Math|Vector|VectorLength NormalImpulse))
  ;[1 1 1] Debris Hit sound
  (if (>= _returnvalue 1e+02)
    (Audio|PlaySoundatLocation (Variables|GlassSettings|GetBreak%20Sound) (.location Hit) "0, 0, 0" (* _returnvalue 0.001) 1.0 0.0 0 0 0)))

(event Custom|FirstHitPositionObject
  (params (FirstPositionBox :type Integer) (TextureY :type Integer) (TextureX :type Integer) (HitPosition :type Vector) (ObjDirection :type Vector) (DamageRadius :type Float%20%28single-precision%29) (FirstHitCanBreakIt :type Boolean) (CharacterVelocityToBreak :type Float%20%28single-precision%29))
  (bind _glass_break_dm_struct (Utilities|Struct|MakeGlass_Break_DM_Struct))
  (bind _damage_radius_multiply (Variables|GlassSettings|GetDamage%20Radius%20Multiply))
  (bind _select_size (Variables|GlassSettings|GetSelect%20Size))
  (bind _sm_glass_dm (Variables|Default|GetSM_Glass_DM))
  (bind _select_size_2 (Variables|GlassSettings|GetSelect%20Size))
  (bind _cast_shadows (Variables|GlassSettings|GetCast%20Shadows))
  (bind (_05x05 _05x05_sh _1x1 _1x1_sh _15x15 _15x15_sh) (Utilities|Struct|BreakGlass_Break_DM_Struct _glass_break_dm_struct))
  (bind (_origin _boxextent _sphereradius) (Collision|GetComponentBounds _sm_glass_dm))
  (bind _returnvalue (* DamageRadius _damage_radius_multiply))
  (bind _returnvalue_2 (Utilities|Select :Index _select_size :NewEnumerator0 2 :NewEnumerator1 3 :NewEnumerator2 4))
  (bind _returnvalue_3 (Utilities|Select :Index _select_size :NewEnumerator0 2 :NewEnumerator1 3 :NewEnumerator2 4))
  (bind _returnvalue_4 (Math|Conversions|ToFloat(Integer) _returnvalue_2))
  (bind _returnvalue_5 (Math|Conversions|ToFloat(Integer) _returnvalue_3))
  (bind _returnvalue_6 (select _cast_shadows _05x05_sh _05x05))
  (bind _returnvalue_7 (select _cast_shadows _1x1_sh _1x1))
  (bind _returnvalue_8 (select _cast_shadows _15x15_sh _15x15))
  (bind _returnvalue_9 (/ 1.0 _returnvalue_4))
  (bind _returnvalue_10 (/ 1.0 _returnvalue_5))
  (bind _output (Utilities|Array|Get(acopy) _returnvalue_6 FirstPositionBox))
  (bind _output_2 (Utilities|Array|Get(acopy) _returnvalue_8 FirstPositionBox))
  (bind _output_3 (Utilities|Array|Get(acopy) _returnvalue_7 FirstPositionBox))
  (bind _returnvalue_11 (Utilities|Select :Index _select_size_2 :NewEnumerator0 _output :NewEnumerator1 _output_3 :NewEnumerator2 _output_2))
  ;[1 1 1] Select destructible mesh to break
  (Utilities|FlowControl|Sequence
    (:then_0
      (if (Variables|GlassSettings|GetAlready%20Broken)
        (Audio|PlaySoundatLocation (Variables|GlassSettings|GetBreak%20Sound) HitPosition "0, 0, 0" 1.0 1.0 0.0 0 0 0)
        (Class|DestructibleComponent|ApplyRadiusDamage (Variables|Default|GetSM_Glass_DM) 5.0 HitPosition _returnvalue 2e+01 false)
        (elif (and FirstHitCanBreakIt (>= CharacterVelocityToBreak (Variables|GlassSettings|GetCharacterVelocityToBreakIt)))
          (if (Utilities|IsValid _returnvalue_11)
            (Utilities|FlowControl|DoOnce false
              (:Completed
                (Class|DestructibleComponent|SetDestructibleMesh (Variables|Default|GetSM_Glass_DM) _returnvalue_11)
                (Components|DestroyComponent (Variables|Default|GetSM_Glass))
                (Class|DestructibleComponent|ApplyRadiusDamage (Variables|Default|GetSM_Glass_DM) 5.0 HitPosition _returnvalue 2e+01 false)
                (Audio|PlaySoundatLocation (Variables|GlassSettings|GetBreak%20Sound) HitPosition "0, 0, 0" 1.0 1.0 0.0 0 0 0)
                (Effects|SpawnEmitteratLocation (Variables|GlassSettings|GetParticles) HitPosition (Math|Rotator|MakeRotfromX ObjDirection))
                (Variables|GlassSettings|SetAlready%20Broken true)
                (Utilities|FlowControl|Sequence
                  (:then_0
                    (if (Variables|TextureSettings|GetGenerate%20Normal%20Maps%20)
                      (bind _returnvalue_12 (Rendering|Material|CreateDynamicMaterialInstance (Variables|Default|GetSM_Glass_DM) (Math|Integer|SelectInt 2 1 (Variables|GlassSettings|GetCast%20Shadows)) (Variables|GlassSettings|GetGlass%20Material) "None" :!class /Script/Engine.PrimitiveComponent))
                      (Rendering|Material|SetScalarParameterValue _returnvalue_12 "Normal_Offset_X" (+ (* (- TextureX 1) _returnvalue_10) (* _returnvalue_10 0.5)) :!class /Script/Engine.MaterialInstanceDynamic)
                      (Rendering|Material|SetScalarParameterValue _returnvalue_12 "Normal_Offset_Y" (+ (* (- TextureY 1) _returnvalue_9) (* _returnvalue_9 0.5)) :!class /Script/Engine.MaterialInstanceDynamic)
                      (Rendering|Material|SetScalarParameterValue _returnvalue_12 "Break_Normal_Intensity" (Variables|TextureSettings|GetBreak%20Normal%20Intensity) :!class /Script/Engine.MaterialInstanceDynamic)
                      (Rendering|Material|SetScalarParameterValue _returnvalue_12 "Cells_Normal_Tile" (Utilities|Select :Index (Variables|GlassSettings|GetSelect%20Size) :NewEnumerator0 0.5 :NewEnumerator1 1.0 :NewEnumerator2 1.5) :!class /Script/Engine.MaterialInstanceDynamic)
                      (Rendering|Material|SetScalarParameterValue _returnvalue_12 "Cells_Normal_Intensity" (Variables|TextureSettings|GetCells%20Normal%20Intensity) :!class /Script/Engine.MaterialInstanceDynamic)))
                  (:then_1
                    (for _array_element (Variables|GlassSettings|GetPositionBoxCollision)
                      (Components|DestroyComponent _array_element))))))))))
    (:then_1
      (Utilities|FlowControl|Delay 3.0)
      (Class|DestructibleComponent|ApplyRadiusDamage (Variables|Default|GetSM_Glass_DM) 5.0 _origin (* _sphereradius 2.0) 1.0 true)
      (Utilities|FlowControl|Delay 2.0)
      (Collision|SetCollisionEnabled (Variables|Default|GetSM_Glass_DM) "NoCollision"))))

(event Custom|Multicast_ExplosiveDamage
  (bind _sm_glass (Variables|Default|GetSM_Glass))
  (bind (_origin _boxextent _sphereradius) (Collision|GetComponentBounds _sm_glass))
  (CallFunction|FirstHitPositionObject 0 0 0 _origin (Math|Vector|GetForwardVector (Variables|Default|GetSM_Glass)) _sphereradius true 1e+04))

(event Custom|ExplosiveDamage
  (CallFunction|MulticastExplosiveDamage))

(fn ConstructionScript
  (bind _select_size (Variables|GlassSettings|GetSelect%20Size))
  (bind _glass_material (Variables|GlassSettings|GetGlass%20Material))
  (bind _select_size_2 (Variables|GlassSettings|GetSelect%20Size))
  (bind _sm_glass (Variables|Default|GetSM_Glass))
  (bind _sm_glass_2 (Variables|Default|GetSM_Glass))
  (bind _returnvalue (Utilities|Select :Index _select_size :NewEnumerator0 2 :NewEnumerator1 3 :NewEnumerator2 4))
  (bind _returnvalue_2 (Utilities|Select :Index _select_size :NewEnumerator0 2 :NewEnumerator1 3 :NewEnumerator2 4))
  (bind _staticmesh (Variables|/Script/Engine.StaticMeshComponent|GetStaticMesh _sm_glass_2))
  (bind _returnvalue_3 (StaticMesh|GetBounds _staticmesh))
  (bind _returnvalue_4 (Math|Conversions|ToFloat(Integer) _returnvalue))
  (bind _returnvalue_5 (Math|Conversions|ToFloat(Integer) _returnvalue_2))
  (bind _returnvalue_6 (* (.boxextent _returnvalue_3) 2))
  (bind (_x _y _z) (Math|Vector|BreakVector _returnvalue_6))
  (bind _returnvalue_7 (/ _y _returnvalue_5))
  (bind _returnvalue_8 (/ _z _returnvalue_4))
  (bind _returnvalue_9 (* _returnvalue_8 0.5))
  (bind _returnvalue_10 (* _returnvalue_7 0.5))
  (Components|StaticMesh|SetStaticMesh (Variables|Default|GetSM_Glass) (select (Variables|GlassSettings|GetCast%20Shadows) (Utilities|Select :Index _select_size_2 :NewEnumerator0 "/Game/BreakableGlass/Meshes/SM_Glass_50x50_Sh.SM_Glass_50x50_Sh" :NewEnumerator1 "/Game/BreakableGlass/Meshes/SM_Glass_100x100_Sh.SM_Glass_100x100_Sh" :NewEnumerator2 "/Game/BreakableGlass/Meshes/SM_Glass_150x150_Sh.SM_Glass_150x150_Sh") (Utilities|Select :Index _select_size_2 :NewEnumerator0 "/Game/BreakableGlass/Meshes/SM_Glass_50x50.SM_Glass_50x50" :NewEnumerator1 "/Game/BreakableGlass/Meshes/SM_Glass_100x100.SM_Glass_100x100" :NewEnumerator2 "/Game/BreakableGlass/Meshes/SM_Glass_150x150.SM_Glass_150x150")))
  (Rendering|Material|SetMaterial (Variables|Default|GetSM_Glass) 0 _glass_material)
  (bind _returnvalue_11 (Rendering|Material|CreateDynamicMaterialInstance _sm_glass 0 _glass_material "None" :!class /Script/Engine.PrimitiveComponent))
  (Rendering|Material|SetMaterial _sm_glass 0 _returnvalue_11)
  (if (Variables|GlassSettings|GetCast%20Shadows)
    (Rendering|Material|SetMaterial _sm_glass 2 _returnvalue_11)
    (bind _returnvalue_12 (Rendering|Material|CreateDynamicMaterialInstance (Variables|Default|GetSM_Glass_DM) 1 "/Game/BreakableGlass/Materials/MI_Shadow.MI_Shadow" "None" :!class /Script/Engine.PrimitiveComponent))
    (Rendering|Material|SetMaterial (Variables|Default|GetSM_Glass) 3 _returnvalue_12)
    (Rendering|Material|SetScalarParameterValue _returnvalue_12 "Shadow Opacity" (Variables|GlassSettings|GetShadow%20Opacity) :!class /Script/Engine.MaterialInstanceDynamic)
    (else
      (Rendering|Material|SetMaterial _sm_glass 1 _returnvalue_11)))
  (for _index (range 0 (- _returnvalue 1))
    (Variables|Default|SetTexture_Y (+ (Variables|Default|GetTexture_Y) 1))
    (for _index_2 (range 0 (- _returnvalue_2 1))
      (if (>= (Variables|Default|GetTexture_X) _returnvalue_2)
        (Variables|Default|SetTexture_X 1)
        (else
          (Variables|Default|SetTexture_X (+ (Variables|Default|GetTexture_X) 1))))
      (Variables|GlassSettings|SetTag_Num (+ (Variables|GlassSettings|GetTag_Num) 1))
      (bind _returnvalue_13 (AddComponent|AddBoxComponent false (Math|Transform|MakeTransform (Math|Vector|MakeVector 0.0 (+ _returnvalue_10 (* _index_2 _returnvalue_7)) (+ (* _index _returnvalue_8) _returnvalue_9)) "0, 0, 0" "1,1,1")))
      (Utilities|Array|Add (Variables|GlassSettings|GetPositionBoxCollision) _returnvalue_13)
      (Rendering|SetVisibility _returnvalue_13 (Variables|GlassSettings|GetShow%20Hit%20Points) true)
      (Variables|/Script/Engine.ActorComponent|SetComponentTags _returnvalue_13 (Utilities|Array|MakeArray (Utilities|String|StringToName (Utilities|String|ToString(Integer) (Variables|GlassSettings|GetTag_Num))) (Utilities|String|StringToName (Utilities|String|ToString(Integer) (Variables|Default|GetTexture_Y))) (Utilities|String|StringToName (Utilities|String|ToString(Integer) (Variables|Default|GetTexture_X)))))
      (Components|Box|SetBoxExtent _returnvalue_13 (Math|Vector|MakeVector 0.0 _returnvalue_10 _returnvalue_9) false))))