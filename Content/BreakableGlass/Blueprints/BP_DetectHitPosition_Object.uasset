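; Child-actor helper that detects where its moving parent object will strike a BP_BreakableGlass and reports the impact to the glass.
; On BeginPlay it sizes a collision-ignoring sphere to the parent's bounds, with a five-second lifetime.
; Each tick it predicts a short projectile path from the sphere's velocity, caching glass hit location and tag-encoded piece indices.
; A gate fires FirstHitPositionObject once the prediction leaves the glass, then the helper destroys itself.
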(event EventTick
  (params (DeltaSeconds :type Float%20%28single-precision%29))
  (bind _returnvalue (Physics|GetPhysicsLinearVelocity (Variables|Default|GetSphere) "None"))
  (bind _output_get (Variables|Default|SetObjDirection _returnvalue))
  (bind _outhit (Class|GameplayStatics|BlueprintPredictProjectilePathbyTraceChannel (Transformation|GetActorLocation) _output_get true (Variables|Default|GetParentActorRad) "ECC_Visibility" true 0 "None" 0.0 5.0 0.1))
  (if (== (Utilities|GetClass (.HitActor (Collision|BreakHitResult _outhit))) "/Game/BreakableGlass/Blueprints/BP_BreakableGlass.BP_BreakableGlass_C")
    (Utilities|FlowControl|Sequence
      (:then_0
        (if (>= (- (Math|Conversions|ToInteger(Byte) (Utilities|String|ToString(Name) (Utilities|Array|Get(acopy) (Variables|/Script/Engine.ActorComponent|GetComponentTags (.HitComponent (Collision|BreakHitResult _outhit)))))) 1) 0)
          (Variables|Default|SetLastValidNum (- (Math|Conversions|ToInteger(Byte) (Utilities|String|ToString(Name) (Utilities|Array|Get(acopy) (Variables|/Script/Engine.ActorComponent|GetComponentTags (.HitComponent (Collision|BreakHitResult _outhit)))))) 1))
          (else
            (Variables|Default|SetLastValidNum (Variables|Default|GetLastValidNum))))
        (Utilities|IsValid (.HitActor (Collision|BreakHitResult _outhit))
          (:Is%20Valid
            (Variables|Default|SetLast%20Valid%20Hit%20Actor (.HitActor (Collision|BreakHitResult _outhit)))
            (Variables|Default|SetLast%20Hit%20Location (.Location (Collision|BreakHitResult _outhit)))
            (Variables|Default|SetLastValidTextureY (Math|Conversions|ToInteger(Byte) (Utilities|String|ToString(Name) (Utilities|Array|Get(acopy) (Variables|/Script/Engine.ActorComponent|GetComponentTags (.HitComponent (Collision|BreakHitResult _outhit))) 1))))
            (Variables|Default|SetLastValidTextureX (Math|Conversions|ToInteger(Byte) (Utilities|String|ToString(Name) (Utilities|Array|Get(acopy) (Variables|/Script/Engine.ActorComponent|GetComponentTags (.HitComponent (Collision|BreakHitResult _outhit))) 2)))))))
      (:then_1
        (goto _label Open)))
    (else
      (Utilities|FlowControl|Gate true :!label _label
        (:Exit
          (Actor|DestroyActor)
          (bind _asbp_breakable_glass (Utilities|Casting|CastToBP_BreakableGlass (Variables|Default|GetLast%20Valid%20Hit%20Actor)))
          (Default|FirstHitPositionObject _asbp_breakable_glass (Variables|Default|GetLastValidNum) (Variables|Default|GetLastValidTextureY) (Variables|Default|GetLastValidTextureX) (Variables|Default|GetLast%20Hit%20Location) (Variables|Default|GetObjDirection) (Variables|Default|GetParentActorRad) true 1e+04))))))

(event EventBeginPlay
  (bind _sphere (Variables|Default|GetSphere))
  (Collision|SetCollisionResponsetoAllChannels _sphere "ECR_Ignore")
  (bind _output_get (Variables|Default|SetParentActorRad (Math|Vector|GetMaxElement (.BoxExtent (Collision|GetActorBounds (Actor|GetParentActor) false false)))))
  (Components|Sphere|SetSphereRadius _sphere _output_get true)
  (Utilities|FlowControl|Delay 5.0)
  (Actor|DestroyActor))

(fn ConstructionScript)