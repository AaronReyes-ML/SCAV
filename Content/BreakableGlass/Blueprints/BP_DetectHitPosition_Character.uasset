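; Character hit detector for breakable glass, reporting where and how fast a moving character strikes a pane.
; Each tick it line-traces along its collision-ignoring Sphere's velocity, accepting hits within the player's capsule radius plus a small margin.
; On BP_BreakableGlass, it decodes the hit component's tags into box index and texture coordinates.
; It passes these to FirstHitPositionObject with hit location, direction, speed and the glass's character-can-break flag.
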(event EventTick
  (params (DeltaSeconds :type Float%20%28single-precision%29))
  (bind _returnvalue (Transformation|GetActorLocation))
  (bind _returnvalue_2 (Physics|GetPhysicsLinearVelocity (Variables|Default|GetSphere) "None"))
  (bind _output_get (Variables|Default|SetObjDirection _returnvalue_2))
  (bind (_outhit _returnvalue_3) (Collision|LineTraceByChannel _returnvalue (+ (Math|Vector|VectorClampSizeMax _output_get 5e+02) _returnvalue) "TraceTypeQuery1" false 0 "None"))
  (if _returnvalue_3
    (if (<= (.Distance (Collision|BreakHitResult _outhit)) (Variables|Default|GetParentActorRad))
      (bind _asbp_breakable_glass (Utilities|Casting|CastToBP_BreakableGlass (.HitActor (Collision|BreakHitResult _outhit))))
      (Default|FirstHitPositionObject _asbp_breakable_glass (- (Math|Conversions|ToInteger(Byte) (Utilities|String|ToString(Name) (Utilities|Array|Get(acopy) (Variables|/Script/Engine.ActorComponent|GetComponentTags (.HitComponent (Collision|BreakHitResult _outhit)))))) 1) (Math|Conversions|ToInteger(Byte) (Utilities|String|ToString(Name) (Utilities|Array|Get(acopy) (Variables|/Script/Engine.ActorComponent|GetComponentTags (.HitComponent (Collision|BreakHitResult _outhit))) 1))) (Math|Conversions|ToInteger(Byte) (Utilities|String|ToString(Name) (Utilities|Array|Get(acopy) (Variables|/Script/Engine.ActorComponent|GetComponentTags (.HitComponent (Collision|BreakHitResult _outhit))) 2))) (.Location (Collision|BreakHitResult _outhit)) (Variables|Default|GetObjDirection) 2.0 (Variables|/Game/BreakableGlass/Blueprints/BP_BreakableGlass.BP_BreakableGlass_C|GetCharacter%20can%20break%20it _asbp_breakable_glass) (Math|Vector|VectorLength _returnvalue_2)))))

(event EventBeginPlay
  (Collision|SetCollisionResponsetoAllChannels (Variables|Default|GetSphere) "ECR_Ignore")
  (Variables|Default|SetParentActorRad (+ (Variables|/Script/Engine.CapsuleComponent|GetCapsuleRadius (Variables|/Script/Engine.Character|GetCapsuleComponent (Game|GetPlayerCharacter 0))) 6.0)))

(fn ConstructionScript)